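; Game mode for a synced PvP mode that creates characters manually after matchmaking.
; With auto-creation off, it opens matchmaking UI, then readies up immediately or via a configurable preparation screen with timeout.
; On battle start it spawns local, remote and AI characters at MiniPlayerStarts matching seat and team, then shows gameplay UI.
; AI types derive from the room's random seed; an empty OnCreateCharacterComplete overrides parent character initialization.
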(event `自定义属性改变`
  (params (PlayerInfo :type "PlayerRoomInfo Structure"))
  (bind (_playerid _seatid _teamid _isai _pvpparam) (break `PlayerRoomInfo` PlayerInfo))
  (bind (_int64param _strparam) (break `PvpStartParam` _pvpparam))
  ;[1 1 1] 需要进入准备阶段
  (`KismetSystemLibrary.PrintText` (`|FormatText` "玩家{playerid}，座位{seatid}，队伍{teamid}，重新设置了整数属性{int64}，字符串属性{str}" _playerid _seatid _teamid (`KismetTextLibrary.Conv_Int64ToText` _int64param) _strparam)))

(event `匹配进入战斗`
  (params (Success :type Boolean) (RoomMsg :type "RoomMsg Structure"))
  (bind _returnvalue (subsystem `BattleMatchSubsystem`))
  (bind (_value _returnvalue_2) (`BlueprintMapLibrary.Map_Find` (`.Map` (break `PVPSceneConfig` (`|GetGameData` "PVP匹配"))) (`TeamSchedulingSubSystem.GetTeamTypeId` (subsystem `TeamSchedulingSubSystem`))))
  (`KismetSystemLibrary.PrintText` (`|FormatText` "匹配进入战斗结果{0}" Success))
  (if Success
    (`GameSubSystem.StartMatch` (subsystem `GameSubSystem`) Success RoomMsg)
    (`KismetSystemLibrary.PrintText` "开始比赛StartMatch")
    ;[1 1 1] 判断准备阶段配置
    (if (and _returnvalue_2 (<= (`.MaxPrepareTime` (break `PVPConfig` _value)) 0))
      (`BattleMatchSubsystem.ReadyToBattle` _returnvalue :!label _label)
      (`KismetSystemLibrary.PrintText` "已准备进入战场Ready to Battle")
      (else
        ;[1 1 1] 需要进入准备阶段
        (bind _returnvalue_3 (`|CreateWidget` "/Game/UI/组队匹配/准备界面.准备界面_C"))
        (`UserWidget.AddToViewport` _returnvalue_3 0)
        (add `BattleMatchSubsystem.BattleReadyTimeoutHandle` _returnvalue (delegate `准备超时事件`))
        (add `BattleMatchSubsystem.BattlePvpParamUpdateHandle` _returnvalue (delegate `自定义属性改变`))))))

(event `self.ReceiveBeginPlay`
  (bind _returnvalue (subsystem `BattleMatchSubsystem`))
  (`parent.ReceiveBeginPlay`)
  (if (not (`self.IsAutoCreateCharacter`))
    (`|ExecutionSequence`
      (:`then_0`
        (`self.打开匹配界面`))
      (:`then_1`
        (add `BattleMatchSubsystem.MatchResultHandle` _returnvalue (delegate `匹配进入战斗`)))
      (:`then_2`
        ;[1 1 1] 开始战斗：创角、UI
        (add `BattleMatchSubsystem.StartBattleHandle` _returnvalue (delegate `开始战斗`))))))

(event `准备超时事件`
  (bind _returnvalue (subsystem `BattleMatchSubsystem`))
  ;[1 1 1] 需要进入准备阶段
  (remove `BattleMatchSubsystem.BattleReadyTimeoutHandle` _returnvalue (delegate `准备超时事件`) :!label _label_2)
  (remove `BattleMatchSubsystem.BattlePvpParamUpdateHandle` _returnvalue (delegate `自定义属性改变`))
  (goto _label))

(event `准备完成事件`
  ;[1 1 1] 需要进入准备阶段
  (goto _label_2))

(event `开始战斗`
  (params (Success :type Boolean) (TimestampNow :type Integer64) (TimestampEnd :type Integer64))
  (bind (_selfinfo _othersinfo _randomseed) (break `RoomMsg` (`BattleMatchSubsystem.GetCurRoomMsg` (subsystem `BattleMatchSubsystem`))))
  ;[1 1 1] 开始战斗：创角、UI
  (`KismetSystemLibrary.PrintText` "收到开始战斗！StartBattle")
  (set `self.Random Seed` _randomseed) ; 保存种子用于随机
  (`self.创建角色` _selfinfo true)
  (for _array_element _othersinfo
    (`self.创建角色` _array_element))
  (`GameSubSystem.StartBattle` (subsystem `GameSubSystem`) Success)
  (bind _returnvalue (`|CreateWidget` "/Game/UI/同步玩法UI.同步玩法UI_C"))
  (`UserWidget.AddToViewport` _returnvalue 0)
  (`/Engine/EditorBlueprintResources/StandardMacros.IsValid` (stale `匹配进入战斗` _returnvalue_3)
    (:`Is Valid`
      (`Widget.RemoveFromParent` (stale `匹配进入战斗` _returnvalue_3))
      (`KismetSystemLibrary.PrintText` "手动创角完成"))))

(event `self.OnCreateCharacterComplete`
  (params (Character :type "MiniGameCharacter Object Reference") (IsMajorPlayer :type Boolean) (IsAI :type Boolean) (PlayerID :type Integer64) (SeatID :type Integer) (TeamID :type Integer) (PvpInterParam :type Integer64) (PvpStrParam :type String)))

(fn `CreateCustomCharacter`
  (params (PvpInterParam :type Integer64) (PvpStrParam :type String))
  (returns (ReturnValue :type "MiniGameCharacter Object Reference"))
  (return null))

(fn `UserConstructionScript`)

(fn `创建角色`
  (params (PlayerRoomInfo :type "PlayerRoomInfo Structure (by ref)") (`是否本地角色` :type Boolean))
  (locals (`生成变换` :type "Transform Structure"))
  (bind (_playerid _seatid _teamid _isai _pvpparam) (break `PlayerRoomInfo` PlayerRoomInfo))
  (bind _random_seed (`self.Random Seed`))
  (bind (_int64param _strparam) (break `PvpStartParam` _pvpparam))
  (bind _returnvalue (`KismetMathLibrary.Conv_IntToInt64` _playerid))
  (bind _returnvalue_2 (`KismetMathLibrary.RandomIntegerInRangeFromStream` 0 2 (`self.种子随机流送`)))
  (`KismetSystemLibrary.PrintText` (`|FormatText` "PlayerID：{0}，SeatID：{1}，TeamID：{2}，是否本地角色：{3}，是否AI：{4}，PVP整数属性：{5}，PVP字符串：{6}" _playerid _seatid _teamid `是否本地角色` _isai (`KismetTextLibrary.Conv_Int64ToText` _int64param) _strparam))
  ;[1 1 1] 根据出生点配置设置生成位置
  (bind _outactors (`GameplayStatics.GetAllActorsOfClass` "/Script/MiniGameProject.MiniPlayerStart"))
  (for _array_element _outactors
    (if (and (== _seatid (`MiniPlayerStart.PlayerSeatID` _array_element)) (== _teamid (`MiniPlayerStart.PlayerTeamID` _array_element)))
      (set `local.生成变换` (`self.GetTransform` _array_element))
      (break)))
  (if `是否本地角色`
    (`self.SetControllerIndex` _seatid)
    ;[1 1 1] 玩家角色
    (bind _returnvalue_3 (`self.CreateCharacter` "/Game/蓝图/Character/BP_同步角色.BP_同步角色_C" (.location (`local.生成变换`)) (.rotation (`local.生成变换`)) _returnvalue _seatid _teamid _int64param _strparam :!label _label))
    (bind `_asbp_同步角色` (cast `/Game/蓝图/Character/BP_同步角色` _returnvalue_3))
    (`/Game/蓝图/Character/BP_同步角色.初始化` `_asbp_同步角色` _seatid _teamid _returnvalue `是否本地角色` _int64param)
    (elif _isai
      ;[1 1 1] AI角色
      (bind _returnvalue_4 (`self.CreateCharacter` "/Game/蓝图/AI/BP_AI.BP_AI_C" (.location (`local.生成变换`)) (.rotation (`local.生成变换`)) _returnvalue _seatid _teamid _int64param _strparam))
      (bind `_asbp_同步角色_2` (cast `/Game/蓝图/Character/BP_同步角色` _returnvalue_4))
      (`KismetMathLibrary.SetRandomStreamSeed` (`self.种子随机流送`) _random_seed)
      (set `self.Random Seed` (+ _random_seed _returnvalue_2)) ; 随机一次之后，重设种子
      (`/Game/蓝图/Character/BP_同步角色.初始化` `_asbp_同步角色_2` _seatid _teamid _returnvalue false (`KismetMathLibrary.Conv_IntToInt64` _returnvalue_2))
      (else
        (goto _label)))))