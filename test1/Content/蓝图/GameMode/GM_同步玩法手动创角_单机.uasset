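; Offline GameMode for the sync gameplay mode (同步玩法), manually spawning a two-versus-two local match.
; BeginPlay starts the local match, creates one player character and three BP_AI at fixed spots, possesses the player, starts the battle and shows the UI.
; The creation-complete callback initializes characters that cast to BP_同步角色 with seat, team and ID, using PvpInterParam as character type and flagging PlayerID 1 as local.
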(event `self.ReceiveBeginPlay`
  (bind _returnvalue (subsystem `GameSubSystem`))
  (`parent.ReceiveBeginPlay`)
  (`GameSubSystem.StartMatchLocalMode` _returnvalue)
  (bind _returnvalue_2 (`self.CreateCharacter` "/Game/蓝图/Character/BP_同步角色.BP_同步角色_C" (612.0 238.0 0.0) (struct :`Yaw` -540.0) 1 1 0))
  (`self.CreateCharacter` "/Game/蓝图/AI/BP_AI.BP_AI_C" (612.0 -238.0 0.0) (struct :`Yaw` -540.0) -1 2 0)
  (`self.CreateCharacter` "/Game/蓝图/AI/BP_AI.BP_AI_C" (-857.0 418.0 0.0) (struct) -2 3 1 1)
  (`self.CreateCharacter` "/Game/蓝图/AI/BP_AI.BP_AI_C" (-857.0 -181.0 0.0) (struct) -3 4 1 2)
  (`Controller.Possess` (`GameplayStatics.GetPlayerController` 0) _returnvalue_2)
  (`GameSubSystem.StartBattleLocalMode` _returnvalue)
  (bind _returnvalue_3 (`|CreateWidget` "/Game/UI/同步玩法UI.同步玩法UI_C"))
  (`UserWidget.AddToViewport` _returnvalue_3 0))

(event `self.OnCreateCharacterComplete`
  (params (Character :type "MiniGameCharacter Object Reference") (IsMajorPlayer :type Boolean) (IsAI :type Boolean) (PlayerID :type Integer64) (SeatID :type Integer) (TeamID :type Integer) (PvpInterParam :type Integer64) (PvpStrParam :type String))
  (bind `_asbp_同步角色` (cast `/Game/蓝图/Character/BP_同步角色` Character))
  (`/Game/蓝图/Character/BP_同步角色.初始化` `_asbp_同步角色` SeatID TeamID PlayerID (== PlayerID 1) PvpInterParam))

(fn `UserConstructionScript`)