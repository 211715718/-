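; GameMode for a synchronized multiplayer mode with automatic character creation.
; On BeginPlay it runs parent logic, adds the 同步玩法UI widget to the viewport and opens the matchmaking screen.
; When character creation completes, it casts to BP_同步角色 and initializes it with seat, team, player, local-player flag and a role type carried in the PvP integer parameter, then prints the details.
; Login-response and battle-start events are empty.
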(event `self.OnLoginRsp`
  (params (bIsSuccess :type Boolean)))

(event `self.ReceiveBeginPlay`
  (`parent.ReceiveBeginPlay`)
  (bind _returnvalue (`|CreateWidget` "/Game/UI/同步玩法UI.同步玩法UI_C"))
  (`UserWidget.AddToViewport` _returnvalue 0)
  (`self.打开匹配界面`))

(event `self.NotifyStartBattle`)

(event `self.OnCreateCharacterComplete`
  (params (Character :type "MiniGameCharacter Object Reference") (IsMajorPlayer :type Boolean) (IsAI :type Boolean) (PlayerID :type Integer64) (SeatID :type Integer) (TeamID :type Integer) (PvpInterParam :type Integer64) (PvpStrParam :type String))
  ;[1 1 1] 自动创角后对角色初始化
  (bind `_asbp_同步角色` (cast `/Game/蓝图/Character/BP_同步角色` Character))
  (`/Game/蓝图/Character/BP_同步角色.初始化` `_asbp_同步角色` SeatID TeamID PlayerID IsMajorPlayer PvpInterParam)
  (`KismetSystemLibrary.PrintText` (`|FormatText` "PlayerID：{0}，SeatID：{1}，TeamID：{2}，是否本地角色：{3}，是否AI：{4}，PVP整数属性：{5}，PVP字符串：{6}" (`KismetTextLibrary.Conv_Int64ToText` PlayerID) SeatID TeamID IsMajorPlayer IsAI (`KismetTextLibrary.Conv_Int64ToText` PvpInterParam) PvpStrParam)))

(fn `UserConstructionScript`)