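; Game mode for synchronized play (同步玩法) that handles matchmaking UI, match end and restart, showing an unlocked mouse on begin play.
; Outside single-player, it opens the team or main matchmaking screen depending on team membership.
; Game end derives the local result from the triggering team, shows the results screen and calls EndBattle on BattleMatchSubsystem.
; Restart picks the single-player test or regular map by checking its own class; login, battle-start and character-creation hooks are empty.
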(event `self.OnLoginRsp`
  (params (bIsSuccess :type Boolean)))

(event `self.ReceiveBeginPlay`
  (`/Game/蓝图/GameMode/蓝图函数库.鼠标显示且不锁定`))

(event `self.NotifyStartBattle`)

(event `self.OnCreateCharacterComplete`
  (params (Character :type "MiniGameCharacter Object Reference") (IsMajorPlayer :type Boolean) (IsAI :type Boolean) (PlayerID :type Integer64) (SeatID :type Integer) (TeamID :type Integer) (PvpInterParam :type Integer64) (PvpStrParam :type String)))

(fn `CreateCustomCharacter`
  (params (PvpInterParam :type Integer64) (PvpStrParam :type String))
  (returns (ReturnValue :type "MiniGameCharacter Object Reference"))
  (return null))

(fn `UserConstructionScript`)

(fn `打开匹配界面`
  (bind _returnvalue (`TeamSchedulingSubSystem.GetIsInATeam` (subsystem `TeamSchedulingSubSystem`)))
  (if (not (`self.IsSinglePlayerMode`))
    (`KismetSystemLibrary.PrintText` (`|FormatText` "是否在队伍里？{0}" _returnvalue))
    (if _returnvalue
      (bind _returnvalue_2 (`|CreateWidget` "/Game/UI/组队匹配/组队匹配界面.组队匹配界面_C"))
      (`UserWidget.AddToViewport` _returnvalue_2 0)
      (else
        (bind _returnvalue_3 (`|CreateWidget` "/Game/UI/组队匹配/匹配主界面.匹配主界面_C"))
        (`UserWidget.AddToViewport` _returnvalue_3 0)))))

(fn `游戏结束`
  (params (`触发者是否胜利` :type Boolean) (`触发玩家角色` :type "/Game/蓝图/Character/BP_同步角色 Object Reference") (`触发队伍` :type Integer))
  (bind `_队伍id` (`/Game/蓝图/Character/BP_同步角色.队伍ID` (`|GetGameData` "本地玩家角色")))
  (`|ExecutionSequence`
    (:`then_0`
      (`KismetSystemLibrary.PrintText` (`|FormatText` "触发者胜利：{触发者}，触发队伍：{触发队伍}，本地队伍：{本地队伍}" `触发者是否胜利` `触发队伍` `_队伍id`)))
    (:`then_1`
      (bind _returnvalue (`|CreateWidget` "/Game/UI/结算界面.结算界面_C" null (select `bool` (== `触发队伍` `_队伍id`) :`false` (not `触发者是否胜利`) :`true` `触发者是否胜利`)))
      (`UserWidget.AddToViewport` _returnvalue 0))
    (:`then_2`
      (`BattleMatchSubsystem.EndBattle` (subsystem `BattleMatchSubsystem`)))))

(fn `重启一局`
  (bind _returnvalue (`GameplayStatics.GetObjectClass` self))
  (if (or (== _returnvalue "/Game/蓝图/GameMode/GM_同步玩法自动创角_单机.GM_同步玩法自动创角_单机_C") (== _returnvalue "/Game/蓝图/GameMode/GM_同步玩法手动创角_单机.GM_同步玩法手动创角_单机_C"))
    (`GameplayStatics.OpenLevelBySoftObjectPtr` "/Game/地图/同步玩法地图_单机测试.同步玩法地图_单机测试")
    (else
      (`GameplayStatics.OpenLevelBySoftObjectPtr` "/Game/地图/同步玩法地图.同步玩法地图"))))