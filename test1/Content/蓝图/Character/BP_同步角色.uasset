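; Player character for a synced team hook game, using fixed-point logic and received user inputs.
; On logic start it spawns an attached hook and its chain; vector input fires the hook along that direction or facing, gated by attachment and cooldown, through skill slot 0.
; Initialization sets team-based camera, control flip, camp, mesh and colored name tag.
; A received variable reports the game result to the game mode.
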(event `self.OnRecUserVector`
  (params (ID :type "EParaID Enum" :default "Jump") (dir :type "FixVector Structure"))
  (bind `_翻转后方向` (`self.控制翻转处理` dir))
  (if (`self.钩子是否依附`)
    (if (`/Engine/BlueprintsBase/FunctionLibrary/函数库_定点数运算.定点数<=定点数` (`FixedLibrary.GetFixVectorDistance` `_翻转后方向` (`FixedLibrary.CreateFixVectorVar` (0.0 0.0 0.0))))
      ;[1 1 1] 默认为角色方向
      (bind _output_get (set `self.发射方向` (`FixedLibrary.GetActorFix64Forward` self)))
      (`self.尝试发射钩爪` _output_get)
      (else
        (`self.尝试发射钩爪` `_翻转后方向`)))))

(event `self.OnRecUserVar`
  (params (ID :type "EParaID Enum" :default "Jump") (var :type "FixVar Structure"))
  ;[1 1 1] 收到参数A，且值为1，表明本角色触发获胜条件
  (switch `EParaID` ID
    (:`A`
      (`self.收到游戏结束` (`/Engine/BlueprintsBase/FunctionLibrary/函数库_定点数运算.相等（定点数）` var (struct :`value` 1.0 :`IntValue` 1000))))))

(event `发射钩爪`
  (bind `_钩子` (`self.钩子`))
  (`FixedLibrary.CancleAttach` `_钩子`)
  (`self.设置钩子依附状态` false)
  (`/Game/蓝图/钩子/BP_钩子.StartMove` `_钩子` (`self.发射方向`)))

(event `self.LogicStart`
  (bind _returnvalue (`|SpawnActorFromClass` "/Game/蓝图/钩子/BP_钩子.BP_钩子_C" (`KismetMathLibrary.MakeTransform` (0.0 0.0 0.0)) "Undefined" "OverrideRootScale" null (`self.钩子位置偏移`)))
  (set `/Game/蓝图/钩子/BP_钩子.MyHoster` self _returnvalue)
  (set `self.钩子` _returnvalue)
  (`self.钩子依附主角`)
  (`self.生成锁链`))

(event `self.LogicUpdate`
  (params (DeltaTime :type "FixVar Structure"))
  (bind `_钩子当前冷却` (`self.钩子当前冷却`))
  (`KismetSystemLibrary.DrawDebugPoint` (`FixedLibrary.GetVectorValue` (`FixedLibrary.GetActorFix64Position` self)) 2.0 (struct :`G` 1.0 :`B` 0.171109 :`A` 1.0) (`FixedLibrary.GetFloatValue` DeltaTime))
  ;[1 1 1] 冷却计算
  (if (`/Engine/BlueprintsBase/FunctionLibrary/函数库_定点数运算.定点数>定点数` `_钩子当前冷却`)
    (bind _output_get (set `self.钩子当前冷却` (`/Engine/BlueprintsBase/FunctionLibrary/函数库_定点数运算.定点数-定点数` `_钩子当前冷却` DeltaTime)))
    (else
      (set `self.钩子当前冷却` (struct)))))

(event `初始化`
  (params (SeatID :type Integer) (TeamID :type Integer) (PlayerID :type Integer64) (`是否本地角色` :type Boolean) (`角色类型` :type Integer64))
  (bind _textwidget (`self.TextWidget`))
  (set `self.座位ID` SeatID)
  (set `self.队伍ID` TeamID)
  (set `self.PlayerID` PlayerID)
  (set `self.是否本地角色` `是否本地角色`)
  (`|ExecutionSequence`
    (:`then_0`
      ;[1 1 1] 设置本地角色
      (`|ExecutionSequence`
        (:`then_0`
          (if (`self.是否本地角色`)
            (`|GameDataVariableSetter` "本地玩家角色" self)))))
    (:`then_1`
      ;[1 1 1] 设置相机旋转
      (bind _output_get (set `self.控制翻转` (== (`self.队伍ID`) 1)))
      (if (not _output_get)
        (`SceneComponent.K2_SetRelativeRotation` (`self.SpringArm`) (struct :`Yaw` 180.0) false false)))
    (:`then_2`
      ;[1 1 1] 设置模型
      (`SkinnedMeshComponent.SetSkinnedAssetAndUpdate` (`self.skeletaMesh`) (`|GetArrayItem` (`|GetGameData` "角色模型数组") (`KismetMathLibrary.Conv_Int64ToInt` `角色类型`)) true))
    (:`then_3`
      ;[1 1 1] 设置阵营
      (switch `int` (`self.队伍ID`)
        (:`0`
          (set `self.Camp` "A"))
        (:`1`
          (set `self.Camp` "B"))))
    (:`then_4`
      (`KismetSystemLibrary.PrintString` (`KismetTextLibrary.Conv_TextToString` (`|FormatText` "PlayerID：{0}，SeatID：{1}，TeamID：{2}，阵营：{3}，是否本地角色：{4}" (`KismetTextLibrary.Conv_Int64ToText` (`self.PlayerID`)) (`self.座位ID`) (`self.队伍ID`) (`|GetEnumeratorNameAsString` (`self.Camp`)) (`self.是否本地角色`)))))
    (:`then_5`
      ;[1 1 1] 设置头顶名字及颜色
      (`KismetSystemLibrary.Delay` 0.1)
      (`TextWidgetComponent.SetText` _textwidget (`KismetTextLibrary.Conv_Int64ToText` PlayerID false false)) ; 设置头顶名字
      (if (not (`self.与本地角色是否同一队伍`))
        (`TextWidgetComponent.SetTextColor` _textwidget (struct :`R` 0.661458 :`G` 0.034451 :`B` 0.034451 :`A` 1.0))))))

(fn `UserConstructionScript`)

(fn `与本地角色是否同一队伍`
  (returns (`是同一队伍` :type Boolean))
  (bind `_本地玩家角色` (`|GetGameData` "本地玩家角色"))
  (`/Engine/EditorBlueprintResources/StandardMacros.IsValid` `_本地玩家角色`
    (:`Is Valid`
      (return (== (`self.队伍ID`) (`/Game/蓝图/Character/BP_同步角色.队伍ID` `_本地玩家角色`))))
    (:`Is Not Valid`
      (`KismetSystemLibrary.PrintString` "找不到本地玩家角色！" true true)
      (return true))))

(fn `尝试发射钩爪`
  (params (`发射方向` :type "FixVector Structure"))
  (returns (`发射成功` :type Boolean))
  (if (`/Engine/BlueprintsBase/FunctionLibrary/函数库_定点数运算.定点数>定点数` (`self.钩子当前冷却`))
    (return false)
    (else
      (set `self.钩子当前冷却` (`self.钩子冷却配置值`))
      (set `self.发射方向` `发射方向`)
      (bind (_reason _returnvalue) (`MiniGame_SkillComponent.PlayActiveSkillWithSlot` (`self.GetMiniGameSkillComp`) 0))
      (`self.发射钩爪`)
      (return true))))

(fn `控制翻转处理`
  (params (`方向` :type "FixVector Structure"))
  (returns (`翻转后方向` :type "FixVector Structure"))
  (locals (`0向量` :type "FixVector Structure"))
  (if (`self.控制翻转`)
    (return (`/Engine/BlueprintsBase/FunctionLibrary/函数库_定点数运算.定点数向量-定点数向量` (`local.0向量`) `方向`))
    (else
      (return `方向`))))

(fn `收到游戏结束`
  (params (`是否胜利` :type Boolean))
  (bind `_asgm_同步玩法游戏模式` (cast `/Game/蓝图/GameMode/GM_同步玩法游戏模式` (`GameplayStatics.GetGameMode`)))
  (`/Game/蓝图/GameMode/GM_同步玩法游戏模式.游戏结束` `_asgm_同步玩法游戏模式` `是否胜利` self (`self.队伍ID`))
  (`KismetSystemLibrary.PrintText` "收到游戏结束！"))

(fn `生成锁链`
  (bind _returnvalue (`|SpawnActorFromClass` "/Game/蓝图/钩子/BP_锁链.BP_锁链_C" (`KismetMathLibrary.MakeTransform` (0.0 0.0 0.0)) "Undefined" "OverrideRootScale" null self (`self.钩子`)))
  (set `self.锁链` _returnvalue))

(fn `设置钩子依附状态`
  (params (`依附状态` :type Boolean))
  (set `self.钩子是否依附` `依附状态`))

(fn `钩子依附主角`
  (`FixedLibrary.AttachTo` (`self.钩子`) self (`self.钩子位置偏移`))
  (`self.设置钩子依附状态` true)
  (`/Game/蓝图/钩子/BP_钩子.StopMove` (`self.钩子`)))