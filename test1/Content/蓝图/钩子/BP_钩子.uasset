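; BP_钩子 is a grappling-hook projectile that flies from its owner, catches a character and drags it back.
; LogicUpdate runs a three-state machine (idle, flying, returning) using fixed-point math and manual collision checks against the character manager's list.
; Flight bounces off hits and turns back on timeout or catch; an empty hook can still catch while returning.
; The catch stays attached until the hook reaches its owner, then detaches.
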(event `self.LogicUpdate`
  (params (DeltaTime :type "FixVar Structure"))
  (bind _myhoster (`self.MyHoster`))
  (`|ExecutionSequence`
    (:`then_0`
      (switch `/Game/蓝图/钩子/钩子状态` (`self.钩子状态`)
        (:`NewEnumerator0`
          (`FixedLibrary.SetActorFix64Forward` self (`FixedLibrary.GetActorFix64Forward` _myhoster))
          (`self.K2_SetActorRotation` (`self.K2_GetActorRotation` _myhoster)))
        (:`NewEnumerator1`
          (`self.更新钩子位置` DeltaTime)
          ;[1 1 1] 飞行中碰撞判定
          (bind _returnvalue (`GameLibrary.GetCharacterMgr` self))
          (bind _returnvalue_2 (`MiniGameCharacterMgr.GetCharList` _returnvalue))
          (for _array_element _returnvalue_2
            (if (== _array_element (`self.MyHoster`))
              _
              (elif (`FixedLibrary.CheckCollision` _array_element self)
                (set `self.钩子状态` "NewEnumerator2")
                (`self.计算飞回方向`)
                (`self.更新钩子位置` (struct))
                (`self.勾中目标处理` _array_element)
                (break))))
          (`self.飞行超时返回判断`))
        (:`NewEnumerator2`
          (`self.计算飞回方向`)
          (`self.更新钩子位置` DeltaTime)
          (if (`FixedLibrary.CheckCollision` self (`self.MyHoster`))
            (`self.钩子返回手中`)
            (else
              ;[1 1 1] 返回时碰撞判定
              (bind _returnvalue_3 (`GameLibrary.GetCharacterMgr` self))
              (bind _returnvalue_4 (`MiniGameCharacterMgr.GetCharList` _returnvalue_3))
              (for _array_element_2 _returnvalue_4
                (`/Engine/EditorBlueprintResources/StandardMacros.IsValid` (`self.钩中对象`) ; 若已有钩中对象，则不再判断
                  (:`Is Valid`
                    (break))
                  (:`Is Not Valid`
                    (if (`FixedLibrary.CheckCollision` _array_element_2 self)
                      (`self.勾中目标处理` _array_element_2)
                      (break))))))))))
    (:`then_1`
      (`KismetSystemLibrary.DrawDebugPoint` (`FixedLibrary.GetVectorValue` (`FixedLibrary.GetActorFix64Position` self)) 2.0 (struct :`R` 1.0 :`G` 0.057456 :`A` 1.0) (`FixedLibrary.GetFloatValue` DeltaTime)))))

(event `self.OnHit`
  (params (HitResult :type "MiniGameHitResult Structure"))
  (bind (_ishit _hitpos _hitnormal _bouncenormal) (`GeometryLibrary.BreakMiniGameHitResult` HitResult))
  (bind (_returnvalue_x _returnvalue_y) (`KismetMathLibrary.BreakVector` (`FixedLibrary.GetVectorValue` _hitpos)))
  (if (`|EnumEquality` (`self.钩子状态`) "NewEnumerator1")
    (`KismetArrayLibrary.Array_Add` (`self.HitPos`) (`FixedLibrary.CreateFixVectorVar` (`KismetMathLibrary.MakeVector` _returnvalue_x _returnvalue_y (`FixedLibrary.GetFloatValue` (`FixedLibrary.GetZ` (`FixedLibrary.GetActorFix64Position` self))))))
    (bind _output_get (set `self.MoveDir` _bouncenormal))
    (`FixedLibrary.SetActorFix64Forward` self _output_get)
    (`GameplayStatics.SpawnEmitterAtLocation` "/LightGame/Art/Effects/Particles/P_FX_Hit_007.P_FX_Hit_007" (`FixedLibrary.GetVectorValue` (`FixedLibrary.GetActorFix64Position` self)))))

(event `self.ReceiveBeginPlay`)

(fn `StartMove`
  (params (moveDir :type "FixVector Structure"))
  (set `self.钩子状态` "NewEnumerator1")
  (bind _output_get (set `self.MoveDir` moveDir))
  (`FixedLibrary.SetActorFix64Forward` self _output_get)
  (set `self.开始飞行时间` (`FixedLibrary.GetCurrentBattleTime` self)))

(fn `StopMove`
  (set `self.钩子状态` "NewEnumerator0"))

(fn `UserConstructionScript`)

(fn `勾中目标处理`
  (params (`钩中对象` :type "Actor Object Reference"))
  (bind _returnvalue (`FixedLibrary.GetActorFix64Position` self))
  ;[1 1 1] 钩中目标
  (bind _output_get (set `self.钩中对象` `钩中对象`))
  (bind _returnvalue_2 (`FixedLibrary.GetActorFix64Position` _output_get))
  (bind _returnvalue_3 (`FixedLibrary.InverseFixTransformLocation` _returnvalue (`FixedLibrary.GetActorFix64Forward` self) _returnvalue_2))
  (bind (_x _y) (`FixedLibrary.BreakFixVector` _returnvalue_3))
  (`FixedLibrary.AttachTo` _output_get self (`FixedLibrary.MakeFixVector` _x _y (struct :`value` -80.0 :`IntValue` -80000))) ; 钩中的目标依附在钩子上
  (`|SpawnActorFromClass` "/Engine/BlueprintsBase/Actor/特效播放器.特效播放器_C" (`self.GetTransform` self) "Undefined" "OverrideRootScale" null "/LightGame/ArtRes/Effects/Particles/P_FX_Hit_003.P_FX_Hit_003")
  (`KismetSystemLibrary.PrintString` (`KismetStringLibrary.Concat_StrStr` "钩子位置" (`FixedLibrary.Fix64VectorToString` _returnvalue) ", 对方位置" (`FixedLibrary.Fix64VectorToString` _returnvalue_2) ", 相对位置" (`FixedLibrary.Fix64VectorToString` _returnvalue_3)) true true (struct :`G` 0.66 :`B` 1.0 :`A` 1.0) 10.0))

(fn `更新钩子位置`
  (params (`间隔时间` :type "FixVar Structure"))
  (bind _movedir (`self.MoveDir`))
  (bind (_x _y) (`FixedLibrary.BreakFixVector` (`/Engine/BlueprintsBase/FunctionLibrary/函数库_定点数运算.定点数向量+定点数向量` (`FixedLibrary.GetActorFix64Position` self) (`/Engine/BlueprintsBase/FunctionLibrary/函数库_定点数运算.定点数向量*定点数` _movedir (`/Engine/BlueprintsBase/FunctionLibrary/函数库_定点数运算.定点数*定点数` `间隔时间` (`self.speed`))))))
  (`FixedLibrary.SetActorFix64Position` self (`FixedLibrary.MakeFixVector` _x _y (`.Z` (`FixedLibrary.BreakFixVector` (`self.钩子相对角色位置`)))))
  (`FixedLibrary.SetActorFix64Forward` self _movedir)
  (return))

(fn `计算飞回方向`
  (set `self.MoveDir` (`/Engine/BlueprintsBase/FunctionLibrary/函数库_定点数运算.规格化` (`/Engine/BlueprintsBase/FunctionLibrary/函数库_定点数运算.定点数向量-定点数向量` (`/Engine/BlueprintsBase/FunctionLibrary/函数库_定点数运算.定点数向量+定点数向量` (`FixedLibrary.GetActorFix64Position` (`self.MyHoster`)) (`self.钩子相对角色位置`)) (`FixedLibrary.GetActorFix64Position` self)))))

(fn `钩子返回手中`
  ;[1 1 1] 碰到主人后，回到未发射状态
  (`FixedLibrary.CancleAttach` (`self.钩中对象`)) ; 取消钩中目标的依附
  (`/Game/蓝图/Character/BP_同步角色.钩子依附主角` (`self.MyHoster`))
  (set `self.钩子状态` "NewEnumerator0")
  (set `self.钩中对象` null)
  (`KismetSystemLibrary.PrintText` (`|FormatText` "回收钩爪时间：{时间}" (`KismetTextLibrary.Conv_DoubleToText` (`self.GetGameTimeSinceCreation`) "HalfToEven"))))

(fn `飞行超时返回判断`
  (locals (`已飞行时间` :type "FixVar Structure"))
  (bind _output_get (set `local.已飞行时间` (`/Engine/BlueprintsBase/FunctionLibrary/函数库_定点数运算.定点数-定点数` (`FixedLibrary.GetCurrentBattleTime` self) (`self.开始飞行时间`))))
  (if (`/Engine/BlueprintsBase/FunctionLibrary/函数库_定点数运算.定点数>=定点数` _output_get (`self.飞行最大时间`))
    (set `self.钩子状态` "NewEnumerator2")))