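; Hook chain actor that draws the chain between the owning player and the hook weapon with beam-style particles.
; Each tick it reads the weapon's hook state, clearing the chain when unfired and redrawing it while flying out or returning.
; The main particle runs from the player to the first hit point, or the hook if none; extra emitters link every hit point to the hook.
; Extra emitters are spawned on demand, then reused by zeroing their endpoints.
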(event `self.ReceiveBeginPlay`
  (bind _mainpartical (`self.MainPartical`))
  (`FXSystemComponent.SetVectorParameter` _mainpartical "start" (0.0 0.0 0.0))
  (`FXSystemComponent.SetVectorParameter` _mainpartical "end" (0.0 0.0 0.0))
  (`FXSystemComponent.SetVectorParameter` _mainpartical "size" (10.0 0.0 0.0)))

(event `self.ReceiveTick`
  (params (DeltaSeconds :type "Float (single-precision)"))
  (switch `/Game/蓝图/钩子/钩子状态` (`/Game/蓝图/钩子/BP_钩子.钩子状态` (`self.OwnerWeapon`))
    (:`NewEnumerator0`
      (`self.ClearChain`))
    (:`NewEnumerator1`
      (`self.SetChain` :!label _label))
    (:`NewEnumerator2`
      (goto _label))))

(fn `ClearChain`
  (bind _mainpartical (`self.MainPartical`))
  (`FXSystemComponent.SetVectorParameter` _mainpartical "start" (0.0 0.0 0.0))
  (`FXSystemComponent.SetVectorParameter` _mainpartical "end" (0.0 0.0 0.0))
  (for _array_element (`self.ParticalList`)
    (`FXSystemComponent.SetVectorParameter` _array_element "start" (0.0 0.0 0.0))
    (`FXSystemComponent.SetVectorParameter` _array_element "end" (0.0 0.0 0.0))))

(fn `Create Chain`)

(fn `SetChain`
  (bind _returnvalue (`self.K2_GetActorLocation` (`self.OwnerWeapon`)))
  (bind _hitpos (`/Game/蓝图/钩子/BP_钩子.HitPos` (`self.OwnerWeapon`)))
  (`self.ClearChain`)
  (`FXSystemComponent.SetVectorParameter` (`self.MainPartical`) "start" (`self.K2_GetActorLocation` (`self.OwnerPlayer`)))
  (if (> (`KismetArrayLibrary.Array_Length` _hitpos) 0)
    (`FXSystemComponent.SetVectorParameter` (`self.MainPartical`) "end" (`FixedLibrary.GetVectorValue` (`|GetArrayItem` _hitpos)))
    (for (_array_element _array_index) (`/Game/蓝图/钩子/BP_钩子.HitPos` (`self.OwnerWeapon`))
      (if (> (`KismetArrayLibrary.Array_Length` (`self.ParticalList`)) _array_index)
        (bind _output (`|GetArrayItem` (`self.ParticalList`) _array_index))
        (bind _returnvalue_2 (`FixedLibrary.GetVectorValue` _array_element))
        (`FXSystemComponent.SetVectorParameter` _output "start" _returnvalue_2)
        (`FXSystemComponent.SetVectorParameter` _output "end" _returnvalue)
        (else
          (bind _returnvalue_3 (`GameplayStatics.SpawnEmitterAtLocation` "/Game/资源/Mesh/FX_Hook.FX_Hook" (0.0 0.0 0.0) (struct) (1.0 1.0 1.0) false))
          (`KismetArrayLibrary.Array_Add` (`self.ParticalList`) _returnvalue_3)
          (`FXSystemComponent.SetVectorParameter` _returnvalue_3 "start" _returnvalue_2)
          (`FXSystemComponent.SetVectorParameter` _returnvalue_3 "end" _returnvalue)
          (`FXSystemComponent.SetVectorParameter` _returnvalue_3 "size" (10.0 0.0 0.0)))))
    (else
      (`FXSystemComponent.SetVectorParameter` (`self.MainPartical`) "end" (`self.K2_GetActorLocation` (`self.OwnerWeapon`))))))

(fn `UserConstructionScript`)